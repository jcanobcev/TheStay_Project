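; Reception bell prop for the hotel that repeatedly plays a sound at its location while the player holds no keys.
; Tick checks Main_Character's NumKeys and uses a DoOnce, reset after a delayed pair of Bombilla_rota sounds, to loop the double cue without overlap.
; Once the key count is nonzero, FirstKeyTaken latches true and no new cues start.
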(event `self.ReceiveTick`
  (params (DeltaSeconds :type "Float (single-precision)"))
  (if (`self.FirstKeyTaken`)
    _
    (elif (== (`/Game/Characters/Main_Character/Main_Character.Num_Keys` (cast `/Game/Characters/Main_Character/Main_Character` (`GameplayStatics.GetPlayerCharacter` 0) :!pure true)) 0.0)
      (`/Engine/EditorBlueprintResources/StandardMacros.DoOnce` false :!label _label
        (:`Completed`
          (`KismetSystemLibrary.Delay` 2.0)
          (`GameplayStatics.PlaySoundAtLocation` "/Game/Sound/Bombillas/Bombilla_rota.Bombilla_rota" (`self.K2_GetActorLocation`) (struct) 1.0 1.0 0.0 null null null)
          (`KismetSystemLibrary.Delay` 0.5)
          (`GameplayStatics.PlaySoundAtLocation` "/Game/Sound/Bombillas/Bombilla_rota.Bombilla_rota" (`self.K2_GetActorLocation`) (struct) 1.0 1.0 0.0 null null null)
          (goto _label :!via `Reset`)))
      (else
        (set `self.FirstKeyTaken` true)))))

(fn `UserConstructionScript`)