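; TV_BP is a television prop that the player can toggle between a black screen and a static screen.
; Its Box overlap enables player input on any actor entering and disables it only when a ThirdPersonCharacter leaves.
; The Interact action drives a FlipFlop that swaps the mesh material, printing a debug string on the black state.
; BeginPlay plays a one-shot sound at the actor's location, independent of the screen state.
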(event `self.ReceiveBeginPlay`
  (`GameplayStatics.PlaySoundAtLocation` null (`self.K2_GetActorLocation`) (struct) 1.0 1.0 0.0 null null null))

(event `InputAction|Interact`
  (params (Key :type "Key Structure"))
  (:`Pressed`
    (`/Engine/EditorBlueprintResources/StandardMacros.FlipFlop`
      (:`A`
        (`PrimitiveComponent.SetMaterial` (`self.StaticMesh`) 0 "/Game/Props/HOTEL_PROPS/TV/Black.Black")
        (`KismetSystemLibrary.PrintString` "Hello"))
      (:`B`
        (`PrimitiveComponent.SetMaterial` (`self.StaticMesh`) 0 "/Game/Props/HOTEL_PROPS/TV/M_Estatica.M_Estatica")))))

(event `self.Box.OnComponentBeginOverlap`
  (params (OverlappedComponent :type "PrimitiveComponent Object Reference") (OtherActor :type "Actor Object Reference") (OtherComp :type "PrimitiveComponent Object Reference") (OtherBodyIndex :type Integer) (bFromSweep :type Boolean) (SweepResult :type "HitResult Structure (by ref)"))
  (`self.EnableInput` (`GameplayStatics.GetPlayerController` 0)))

(event `self.Box.OnComponentEndOverlap`
  (params (OverlappedComponent :type "PrimitiveComponent Object Reference") (OtherActor :type "Actor Object Reference") (OtherComp :type "PrimitiveComponent Object Reference") (OtherBodyIndex :type Integer))
  (cast `/Game/ThirdPersonBP/Blueprints/ThirdPersonCharacter` OtherActor)
  (`self.DisableInput` null))

(fn `UserConstructionScript`)