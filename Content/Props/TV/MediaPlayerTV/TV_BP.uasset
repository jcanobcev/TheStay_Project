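; Interactive TV prop Blueprint that toggles its screen on and off with the Interact input.
; A FlipFlop alternates between applying a screen material while opening a media source in the MediaPlayer, and swapping to a black material without stopping playback.
; Box overlaps gate input: any begin overlap enables it before the character cast, while end overlap calls DisableInput only for ThirdPersonCharacter.
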(event `InputAction|Interact`
  (params (Key :type "Key Structure"))
  (:`Pressed`
    (`/Engine/EditorBlueprintResources/StandardMacros.FlipFlop`
      (:`A`
        (`PrimitiveComponent.SetMaterial` (`self.StaticMesh`) 0 "/Game/Props/TV/Material__20.Material__20")
        (`MediaPlayer.OpenSource` (`self.MediaPlayer`) "/Game/Props/TV/MediaPlayerTV/aaaa.aaaa"))
      (:`B`
        (`PrimitiveComponent.SetMaterial` (`self.StaticMesh`) 0 "/Game/Props/TV/Black.Black")))))

(event `self.Box.OnComponentBeginOverlap`
  (params (OverlappedComponent :type "PrimitiveComponent Object Reference") (OtherActor :type "Actor Object Reference") (OtherComp :type "PrimitiveComponent Object Reference") (OtherBodyIndex :type Integer) (bFromSweep :type Boolean) (SweepResult :type "HitResult Structure (by ref)"))
  (`self.EnableInput` (`GameplayStatics.GetPlayerController` 0))
  (cast `/Game/ThirdPersonBP/Blueprints/ThirdPersonCharacter` OtherActor))

(event `self.Box.OnComponentEndOverlap`
  (params (OverlappedComponent :type "PrimitiveComponent Object Reference") (OtherActor :type "Actor Object Reference") (OtherComp :type "PrimitiveComponent Object Reference") (OtherBodyIndex :type Integer))
  (cast `/Game/ThirdPersonBP/Blueprints/ThirdPersonCharacter` OtherActor)
  (`self.DisableInput` null))

(fn `UserConstructionScript`)