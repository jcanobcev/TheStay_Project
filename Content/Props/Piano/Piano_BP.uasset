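; Interactive piano prop that reacts to E presses while the player's Main_Character is inside its Box trigger.
; Overlap events toggle input and switch the linked Billboard_Text prompt between its close and far states.
; A counter steps through two placeholder sound prints, then locks at -1 as a timeline rotates the lid closed.
; That timeline's update also destroys the billboard, and its finish prints a placeholder thud sound.
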(event `Key|E`
  (params (Key :type "Key Structure"))
  (:`Pressed`
    (switch `int` (`self.Cont`)
      (:`0`
        (`KismetSystemLibrary.PrintString` "Sonido 1")
        (`/Engine/EditorBlueprintResources/StandardMacros.IncrementInt` (`self.Cont`)))
      (:`1`
        (`KismetSystemLibrary.PrintString` "Sonido 2")
        (`/Engine/EditorBlueprintResources/StandardMacros.IncrementInt` (`self.Cont`)))
      (:`2`
        (`KismetSystemLibrary.PrintString` "Animacion de cerrarse la tapa")
        (set `self.Cont` -1)
        (bind (_direction _newtrack_0) (`Timeline|Close_Piano`)
          (:`Update`
            (`SceneComponent.K2_SetRelativeRotation` (`self.r`) (`KismetMathLibrary.MakeRotator` (`KismetMathLibrary.Lerp` (`self.Tapa_Abierta`) (`self.Tapa_Cerrada`) _newtrack_0)) false false)
            (`self.K2_DestroyActor` (`self.As_Billboard`)))
          (:`Finished`
            (`KismetSystemLibrary.PrintString` "Sonido golpe")))))))

(event `self.ReceiveBeginPlay`
  (bind _asbillboard_text (cast `/Game/Interface/Billboard_Text` (`self.Billboard_Text`)))
  (set `self.As_Billboard` _asbillboard_text))

(event `self.Box.OnComponentBeginOverlap`
  (params (OverlappedComponent :type "PrimitiveComponent Object Reference") (OtherActor :type "Actor Object Reference") (OtherComp :type "PrimitiveComponent Object Reference") (OtherBodyIndex :type Integer) (bFromSweep :type Boolean) (SweepResult :type "HitResult Structure (by ref)"))
  (bind _asmain_character (cast `/Game/Characters/Main_Character/Main_Character` OtherActor))
  (`/Engine/EditorBlueprintResources/StandardMacros.IsValid` _asmain_character
    (:`Is Valid`
      (`self.EnableInput` (`GameplayStatics.GetPlayerController` 0))
      (`/Game/Interface/Billboard_Text.Activate_Close_Colldier_Interactuable` (`self.As_Billboard`)))))

(event `self.Box.OnComponentEndOverlap`
  (params (OverlappedComponent :type "PrimitiveComponent Object Reference") (OtherActor :type "Actor Object Reference") (OtherComp :type "PrimitiveComponent Object Reference") (OtherBodyIndex :type Integer))
  (bind _asmain_character (cast `/Game/Characters/Main_Character/Main_Character` OtherActor))
  (`/Engine/EditorBlueprintResources/StandardMacros.IsValid` _asmain_character
    (:`Is Valid`
      (`self.DisableInput` (`GameplayStatics.GetPlayerController` 0))
      (`/Game/Interface/Billboard_Text.Activate_Far_Collider_Interactuable` (`self.As_Billboard`)))))

(fn `UserConstructionScript`)