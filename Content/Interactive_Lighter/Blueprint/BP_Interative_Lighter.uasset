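; Interactive lighter actor that opens, closes, ignites and can be recolored, with sound, sparks, flame and point light.
; One timeline, played forward or reversed, drives the lid through the Anim Blueprint, while another drives ignition.
; Tick tilts the flame by player velocity direction, shrinking and dimming it with stronger flicker while moving.
; Construction creates dynamic materials for the body and the flickering light function.
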(event `Change Color`
  (params (Color :type "Float (double-precision)"))
  (bind (_h _s _v _a) (`KismetMathLibrary.RGBToHSV` (`self.Color`)))
  ;[1 1 1] Change Lighter Color
  (`MaterialInstanceDynamic.SetVectorParameterValue` (`self.Instanced Lighter Material`) "Color" (`KismetMathLibrary.HSVToRGB` Color _s _v _a)))

(event `self.ReceiveBeginPlay`
  ;[1 1 1] Initializing Values
  (bind _asabp_interactive_lighter (cast `/Game/Interactive_Lighter/Blueprint/ABP_Interactive_Lighter` (`SkeletalMeshComponent.GetAnimInstance` (`self.Interactive Lighter Mesh`))))
  (set `self.ABP Ref` _asabp_interactive_lighter)
  (`KismetSystemLibrary.ExecuteConsoleCommand` "r.Mobile.TonemapperFilm 1" null))

(event `Close Lighter`
  (bind _returnvalue (`self.K2_GetActorLocation`))
  ;[1 1 1] Open & Close Lighter
  (set `self.Can Ignite` false)
  (if (`self.Lighter Is Open`)
    (bind (_direction _alpha) (`Timeline|Lighter Open` :!via `PlayFromStart` :!label _label)
      (:`Update`
        (set `/Game/Interactive_Lighter/Blueprint/ABP_Interactive_Lighter.Open/Close Angle` (`KismetMathLibrary.Lerp` 0.0 -163.0 _alpha) (`self.ABP Ref`))
        (switch `ETimelineDirection` _direction
          (:`Forward`
            (set `self.Lighter Is Open` false)
            (`SceneComponent.SetVisibility` (`self.PointLight`) false false)
            (`SceneComponent.SetVisibility` (`self.Flame`) false false))
          (:`Backward`
            (set `self.Lighter Is Open` true))))
      (:`Finished`
        (switch `ETimelineDirection` _direction
          (:`Forward`
            (`GameplayStatics.PlaySoundAtLocation` "/Game/Interactive_Lighter/Sound/SFX_Lighter_Open_Close_Cue.SFX_Lighter_Open_Close_Cue" _returnvalue (struct) 1.0 1.0 0.0 null null null))
          (:`Backward`
            (set `self.Can Ignite` true)
            (`GameplayStatics.PlaySoundAtLocation` "/Game/Interactive_Lighter/Sound/SFX_Lighter_Open_Close_Cue.SFX_Lighter_Open_Close_Cue" _returnvalue (struct) 1.0 1.0 0.0 null null null)))))))

(event `Open Lighter`
  ;[1 1 1] Open & Close Lighter
  (if (not (`self.Lighter Is Open`))
    (goto _label :!via `ReverseFromEnd`)))

(event `Ignite Lighter`
  ;[1 1 1] Ignite The Lighter
  (`KismetSystemLibrary.Delay` 0.3)
  (if (`self.Can Ignite`)
    (bind (_direction _alpha) (`Timeline|Ignite Lighter Alpha` :!via `PlayFromStart`)
      (:`Update`
        (set `/Game/Interactive_Lighter/Blueprint/ABP_Interactive_Lighter.Ignite Lighter` (`KismetMathLibrary.Lerp` 0.0 180.0 _alpha) (`self.ABP Ref`))
        (`SceneComponent.SetRelativeScale3D` (`self.Flame`) (`KismetMathLibrary.MakeVector` 1.0 1.0 (`KismetMathLibrary.Lerp` 0.0 1.0 _alpha)))
        (`ActorComponent.ToggleActive` (`self.P_Sparks`))
        (`SceneComponent.SetVisibility` (`self.PointLight`) true false)
        (`SceneComponent.SetVisibility` (`self.Flame`) true false))
      (:`Finished`
        (`GameplayStatics.PlaySoundAtLocation` "/Game/Interactive_Lighter/Sound/SFX_Lighter_Ignite_Cue.SFX_Lighter_Ignite_Cue" (`self.K2_GetActorLocation`) (struct) 1.0 1.0 0.0 null null null)))))

(event `self.ReceiveTick`
  (params (DeltaSeconds :type "Float (single-precision)"))
  (bind _returnvalue (`GameplayStatics.GetPlayerCharacter` 0))
  (bind _returnvalue_2 (`GameplayStatics.GetWorldDeltaSeconds`))
  (bind _flame (`self.Flame`))
  (bind _pointlight (`self.PointLight`))
  (bind _flame_max_rotation (`self.Flame Max Rotation`))
  (bind _returnvalue_3 (`self.GetVelocity` _returnvalue))
  (bind (_relativerotation_roll _relativerotation_pitch) (`KismetMathLibrary.BreakRotator` (`SceneComponent.RelativeRotation` _flame)))
  (bind _returnvalue_4 (`KismetMathLibrary.Normal` _returnvalue_3))
  (bind _returnvalue_5 (> (`KismetMathLibrary.VSize` _returnvalue_3) 0.0))
  ;[1 1 1] Flame Behaviour While Moving
  (`/Engine/EditorBlueprintResources/StandardMacros.IsValid` _returnvalue
    (:`Is Valid`
      (`SceneComponent.K2_SetRelativeRotation` _flame (`KismetMathLibrary.MakeRotator` (`KismetMathLibrary.FInterpTo` _relativerotation_roll (* (`KismetMathLibrary.Dot_VectorVector` _returnvalue_4 (`self.GetActorRightVector`)) -1.0 _flame_max_rotation) _returnvalue_2 6.0) (`KismetMathLibrary.FInterpTo` _relativerotation_pitch (* (`KismetMathLibrary.Dot_VectorVector` _returnvalue_4 (`self.GetActorForwardVector`)) _flame_max_rotation) _returnvalue_2 6.0)) false false)
      (`SceneComponent.SetRelativeScale3D` _flame (`KismetMathLibrary.VInterpTo` (`SceneComponent.RelativeScale3D` _flame) (select `bool` _returnvalue_5 :`false` (1.0 1.0 1.0) :`true` (0.8 0.8 0.8) :!type "Vector Structure") _returnvalue_2 6.0))
      (`LightComponent.SetIntensity` _pointlight (`KismetMathLibrary.FInterpTo` (`LightComponentBase.Intensity` _pointlight) (`KismetMathLibrary.SelectFloat` (`self.Minimum Intensity`) (`self.Maximum Intensity`) _returnvalue_5) _returnvalue_2 6.0))
      (`MaterialInstanceDynamic.SetScalarParameterValue` (`self.Light Function`) "Light Flickering" (`KismetMathLibrary.SelectFloat` (`self.Max Flickering Percentage`) (`self.Min Flickering Percentage`) _returnvalue_5)))))

(fn `UserConstructionScript`
  (bind _returnvalue (`PrimitiveComponent.CreateDynamicMaterialInstance` (`self.Interactive Lighter Mesh`) 0 "/Game/Interactive_Lighter/Materials/M_Lighter.M_Lighter" "None"))
  (bind _output_get (set `self.Instanced Lighter Material` _returnvalue))
  (bind _returnvalue_2 (`KismetMaterialLibrary.CreateDynamicMaterialInstance` "/Game/Interactive_Lighter/Materials/M_Flickering_Light.M_Flickering_Light"))
  (bind _output_get_2 (set `self.Light Function` _returnvalue_2))
  (`LightComponent.SetLightFunctionMaterial` (`self.PointLight`) _output_get_2)
  ;[0.1275 0.6198 0.03551] Lighter Material Properties
  (`MaterialInstanceDynamic.SetVectorParameterValue` _output_get "Color" (`self.Color`))
  (`MaterialInstanceDynamic.SetVectorParameterValue` _output_get "Dirt Color" (`self.Dirt Color`))
  (`MaterialInstanceDynamic.SetScalarParameterValue` _output_get "Paint Roughness" (`self.Paint Roughness`))
  (`MaterialInstanceDynamic.SetScalarParameterValue` _output_get "Dirt Roughness" (`self.Dirt Roughness`))
  ;[1 0.5495 0] Light Properties
  (`PointLightComponent.SetAttenuationRadius` (`self.PointLight`) (`self.Light Area Radius`)))