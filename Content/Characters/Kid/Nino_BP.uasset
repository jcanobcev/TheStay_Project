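; Nino_BP is a kid character that follows the player while a movement flag in the game instance is on.
; Each tick it reads Movimiento from GI_IAMap, then sets a walk speed and issues AIMoveTo toward the player's ThirdPersonCharacter.
; When the flag is off, it issues AIMoveTo to its own location, effectively holding it in place.
; BeginPlay also enables input from the first player controller.
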(event `self.ReceiveBeginPlay`
  (`self.EnableInput` (`GameplayStatics.GetPlayerController` 0)))

(event `self.ReceiveTick`
  (params (DeltaSeconds :type "Float (single-precision)"))
  (bind _asgi_iamap (cast `/Game/GI_IAMap` (`GameplayStatics.GetGameInstance`)))
  (if (`/Game/GI_IAMap.Movimiento` _asgi_iamap)
    (bind _asthird_person_character (cast `/Game/ThirdPersonBP/Blueprints/ThirdPersonCharacter` (`GameplayStatics.GetPlayerCharacter` 0)))
    (set `CharacterMovementComponent.MaxWalkSpeed` 140.0 (`self.CharacterMovement`))
    (`|AIMoveTo` (`self.Mesh`) self (`self.K2_GetActorLocation` _asthird_person_character) null)
    (else
      (cast `/Game/ThirdPersonBP/Blueprints/ThirdPersonCharacter` (`GameplayStatics.GetPlayerCharacter` 0))
      (`|AIMoveTo` self (`self.K2_GetActorLocation` self) null 20.0))))

(fn `UserConstructionScript`)